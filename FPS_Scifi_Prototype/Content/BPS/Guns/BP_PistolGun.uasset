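; BP_PistolGun is a pistol weapon Blueprint that fires projectiles.
; Fire spawns a half-scale BP_PistolProjectile at the skeletal mesh's muzzle socket, always spawning regardless of collision.
; A CanFire flag and a FireRateCooldown delay limit the rate of fire.
; StopFire only clears IsFiring, which the Fire logic does not read.
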(event `Fire`
  (bind (_returnvalue_location _returnvalue_rotation) (`KismetMathLibrary.BreakTransform` (`SceneComponent.GetSocketTransform` (`self.SkeletalMesh`) "muzzle" "RTS_World")))
  (if (`self.canFire`)
    (`|SpawnActorFromClass` "/Game/BPS/Projectiles/BP_PistolProjectile.BP_PistolProjectile_C" (`KismetMathLibrary.MakeTransform` _returnvalue_location _returnvalue_rotation (0.5 0.5 0.5)) "AlwaysSpawn" "MultiplyWithRoot" null null)
    (set `self.canFire` false)
    (`KismetSystemLibrary.Delay` (`self.fireRateCooldown`))
    (set `self.canFire` true)))

(event `StopFire`
  (set `self.isFiring` false))

(fn `UserConstructionScript`)