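; BP_Pistol is a gun Blueprint that fires BP_PistolProjectile actors from its skeletal mesh's muzzle socket.
; Fire sets IsFiring and spawns a half-scale projectile, then in automatic mode loops through a retriggerable FireRate delay with a debug print.
; StopFire clears IsFiring, but the flag is checked only after each spawn, so a pending delay still releases one more shot.
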(event `Fire`
  (bind (_returnvalue_location _returnvalue_rotation) (`KismetMathLibrary.BreakTransform` (`SceneComponent.GetSocketTransform` (`self.SkeletalMesh`) "muzzle" "RTS_World")))
  (set `self.isFiring` true)
  (`|SpawnActorFromClass` "/Game/BPS/Projectiles/BP_PistolProjectile.BP_PistolProjectile_C" (`KismetMathLibrary.MakeTransform` _returnvalue_location _returnvalue_rotation (0.5 0.5 0.5)) "AlwaysSpawn" "MultiplyWithRoot" null null :!label _label)
  (if (`self.isAutomatic`)
    (if (`self.isFiring`)
      (`KismetSystemLibrary.PrintString` "Shooting!")
      (`KismetSystemLibrary.RetriggerableDelay` (`self.fireRate`))
      (goto _label))))

(event `StopFire`
  (set `self.isFiring` false))

(fn `UserConstructionScript`)